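; Floating enemy AI that runs a behavior tree and can be knocked around by physics impulses.
; On BeginPlay it starts BT_FloatingEnemyAI through its AI controller, then caches the health widget and hands it a reference to itself.
; The BPI physics impulse event enables simulation on the capsule, applies the impulse at the hit location, and uses a timer to switch simulation off after the given time.
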(event Custom|ResetPhysics
  ;[0.3093 1 0.2107] BPI PHYSICS IMPULSE
  (Physics|SetSimulatePhysics (Variables|Collision|GetCapsuleComponent) false))

(event EventBeginPlay
  (bind _self self)
  (bind _returnvalue (AI|GetAIController _self))
  ;[1 0.1562 0.1562] BEGIN PLAY RUN BEHAVIOUR TREE
  (Utilities|IsValid _returnvalue
    (:Is%20Valid
      (AI|RunBehaviorTree _returnvalue "/Game/BP_EnemyAI/BT_FloatingEnemyAI.BT_FloatingEnemyAI")
      (bind _aswbp_enemy_health (Utilities|Casting|CastToWBP_EnemyHealth (UserInterface|GetUserWidgetObject (Variables|Default|GetEnemyHealth))))
      (bind _output_get (Variables|Default|SetEnemyHealthBar _aswbp_enemy_health))
      (Variables|/Game/WBP_HUD/WBP_EnemyHealth.WBP_EnemyHealth_C|SetFloatingEnemyAI _output_get self))))

(event Collision|EventActorBeginOverlap
  (params (OtherActor :type Actor%20Object%20Reference)))

(event EventTick
  (params (DeltaSeconds :type Float%20%28single-precision%29)))

(event EventBPIPhysicsImpulse
  (params (PhysicsTime :type Float%20%28double-precision%29) (NormalImpulse :type Vector :default "0, 0, 0") (HitLocation :type Vector :default "0, 0, 0"))
  ;[0.3093 1 0.2107] BPI PHYSICS IMPULSE
  (Physics|SetSimulatePhysics (Variables|Collision|GetCapsuleComponent) true)
  (Physics|AddImpulseatLocation (Variables|Collision|GetCapsuleComponent) NormalImpulse HitLocation "None")
  (Utilities|Time|SetTimerbyEvent (delegate Custom|ResetPhysics) PhysicsTime))

(fn ConstructionScript)