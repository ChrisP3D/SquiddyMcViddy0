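; Actor that shows pooled floating text, such as energy gains, as 3D widgets around the player.
; BeginPlay pre-creates hidden WBP_FloatingText widget components and starts a timer that periodically moves the actor to the player.
; SpawnWidget takes an unused component, sets its text, color and location, then attaches it to the player pawn's root.
; Tick turns active widgets toward the camera, and the rise animation's end hides them and frees them for reuse.
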(event Custom|CheckPlayerLocation
  ;[1 1 1] CHECK PLAYER LOCATION EVERY 3S TO MAKE SURE WIDGET IS SPAWNED SOMEWHERE NEARBY
  (Transformation|SetWorldLocation (Variables|Default|GetDefaultSceneRoot) (Transformation|GetWorldLocation (Variables|/Script/Engine.Actor|GetRootComponent (Game|Player|GetPlayerPawn 0))) false false))

(event Custom|SetSpawnWidgetData
  (params (SpawnedWidget :type Widget%20Component%20Object%20Reference) (InText :type Text) (InColorAndOpacity :type Slate%20Color%20Structure))
  ;[1 1 1] SPAWNED WIDGET GETS TEXT AND COLOR INFO, SETS VISIBILITY TO ZERO WHEN ANIMATION FINISHES
  (bind _aswbp_floating_text (Utilities|Casting|CastToWBP_FloatingText (UserInterface|GetWidget SpawnedWidget)))
  (Default|SetEnergyGain _aswbp_floating_text InText InColorAndOpacity)
  (EventDispatchers|AssignOnAnimationFinishedRise _aswbp_floating_text (delegate Custom|OnAnimationFinishedRise_Event)))

(event Custom|MakeFloatingText
  ;[1 1 1] INITIALIZE SETTINGS FOR THE WIDGET
  (bind _returnvalue (Game|AddComponentbyClass "/Script/UMG.WidgetComponent" false))
  (bind _returnvalue_2 (UserInterface|CreateWidget "/Game/WBP_HUD/WBP_FloatingText.WBP_FloatingText_C" 0 _returnvalue))
  (Collision|SetCollisionEnabled _returnvalue "NoCollision")
  (Rendering|Material|SetMaterial _returnvalue 0 "/Engine/EngineMaterials/Widget3DPassThrough_Masked.Widget3DPassThrough_Masked")
  (UserInterface|SetWidget _returnvalue _returnvalue_2)
  (Utilities|Array|Add (Variables|Default|GetFloatingTextComponents) _returnvalue)
  (Rendering|SetVisibility _returnvalue false false)
  ;[1 1 1] CHECK PLAYER LOCATION EVERY 3S TO MAKE SURE WIDGET IS SPAWNED SOMEWHERE NEARBY
  (Transformation|SetWorldLocation (Variables|Default|GetDefaultSceneRoot) (Transformation|GetWorldLocation (Variables|/Script/Engine.Actor|GetRootComponent (Game|Player|GetPlayerPawn 0))) false false))

(event Custom|OnAnimationFinishedRise_Event
  (params (ThisComponent :type Widget%20Component%20Object%20Reference))
  ;[1 1 1] SPAWNED WIDGET GETS TEXT AND COLOR INFO, SETS VISIBILITY TO ZERO WHEN ANIMATION FINISHES
  (Utilities|Array|RemoveItem (Variables|Default|GetSpawnedFloatingTextComponents) ThisComponent)
  (Rendering|SetVisibility ThisComponent false false))

(event EventBeginPlay
  (for _index (range 0 (Variables|Default|GetPoolMax))
    (CallFunction|MakeFloatingText)
    ;[1 1 1] CHECK PLAYER LOCATION EVERY 3S TO MAKE SURE WIDGET IS SPAWNED SOMEWHERE NEARBY
    (Utilities|Time|SetTimerbyEvent (delegate Custom|CheckPlayerLocation) 3.0 true))
  (Transformation|SetWorldLocation (Variables|Default|GetDefaultSceneRoot) (Transformation|GetWorldLocation (Variables|/Script/Engine.Actor|GetRootComponent (Game|Player|GetPlayerPawn 0))) false false))

(event EventTick
  (params (DeltaSeconds :type Float%20%28single-precision%29))
  ;[1 1 1] ENSURE WIDGET ALWAYS FACES PLAYER
  (for _array_element (Variables|Default|GetSpawnedFloatingTextComponents)
    (Transformation|SetWorldRotation _array_element (Math|Rotator|FindLookatRotation (Transformation|GetWorldLocation _array_element) (Camera|GetCameraLocation (Game|GetPlayerCameraManager 0))) false false)))

(fn ConstructionScript)

(fn SpawnWidget
  (params (InText :type Text) (NewLocation :type Vector) (InColorAndOpacity :type Slate%20Color%20Structure))
  (Utilities|FlowControl|Sequence
    (:then_0
      (for _array_element (Variables|Default|GetFloatingTextComponents)
        (if (not (Utilities|Array|ContainsItem (Variables|Default|GetSpawnedFloatingTextComponents) _array_element))
          (LocalVariables|SetWidgetToSpawn _array_element))))
    (:then_1
      (Utilities|IsValid (LocalVariables|GetWidgetToSpawn)
        (:Is%20Valid
          (Utilities|FlowControl|Sequence
            (:then_0
              (CallFunction|SetSpawnWidgetData (LocalVariables|GetWidgetToSpawn) InText InColorAndOpacity))
            (:then_1
              (Utilities|Array|Add (Variables|Default|GetSpawnedFloatingTextComponents) (LocalVariables|GetWidgetToSpawn)))
            (:then_2
              (Transformation|SetWorldLocation (LocalVariables|GetWidgetToSpawn) NewLocation false false))
            (:then_3
              (Rendering|SetVisibility (LocalVariables|GetWidgetToSpawn) true false)
              (Transformation|AttachComponentToComponent (LocalVariables|GetWidgetToSpawn) (Variables|/Script/Engine.Actor|GetRootComponent (Game|Player|GetPlayerPawn 0)) "None" "KeepRelative" "KeepRelative" "KeepRelative" true))))))))