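; BP_StartLevelPawn is the pawn that sets up the start level with MIDI input and the start menu.
; On BeginPlay it spawns a BP_MIDI_Input actor owned by itself, then adds WBP_StartMenu to the viewport and shows the mouse cursor.
; A debug key looks up the BP_MIDI_Input actor and prints each of its device names.
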(event EventBeginPlay
  (Utilities|FlowControl|Sequence
    (:then_0
      (Game|SpawnActorfromClass "/Game/BP_MIDI_Input/BP_MIDI_Input.BP_MIDI_Input_C" (Math|Transform|MakeTransform "0, 0, 0" "0, 0, 0" "1.000000,1.000000,1.000000") "AlwaysSpawn" "MultiplyWithRoot" self 0))
    (:then_1
      (bind _returnvalue (UserInterface|CreateWidget "/Game/Widgets/WBP_StartMenu.WBP_StartMenu_C"))
      (UserInterface|Viewport|AddtoViewport _returnvalue 0)
      (Variables|/Script/Engine.PlayerController|SetbShowMouseCursor (Game|GetPlayerController 0) true))))

(event Collision|EventActorBeginOverlap
  (params (OtherActor :type Actor%20Object%20Reference)))

(event EventTick
  (params (DeltaSeconds :type Float%20%28single-precision%29)))

(event Input|KeyboardEvents|DebugKey1
  (params (Key :type Key%20Structure :default "None") (ActionValue :type Input%20Action%20Value%20Structure))
  (:Pressed
    (bind _returnvalue (Actor|GetActorOfClass "/Game/BP_MIDI_Input/BP_MIDI_Input.BP_MIDI_Input_C"))
    (for _array_element (Variables|/Game/BP_MIDI_Input/BP_MIDI_Input.BP_MIDI_Input_C|GetDeviceNames _returnvalue)
      (Development|PrintString _array_element))))

(fn ConstructionScript)