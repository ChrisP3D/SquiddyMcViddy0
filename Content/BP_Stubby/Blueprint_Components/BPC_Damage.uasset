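; BPC_Damage is a Blueprint component for Stubby that applies a set damage amount to its own owner when TakeDamage fires.
; It subtracts DamageAmount from the owner's BPC_Health, then refreshes the WBP_EnemyHealth widget and calls BPC_Death's Death.
; Sibling components are found by class lookup; Death runs on every hit without a health check here.
; The widget refresh requires BPC_Death, and Death requires a valid widget.
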(event Custom|TakeDamage
  (bind _owner (Variables|Default|GetOwner))
  (bind _owner_2 (Variables|Default|GetOwner))
  (bind _returnvalue (Actor|GetComponentbyClass _owner_2 "/Game/BP_Stubby/Blueprint_Components/BPC_Death.BPC_Death_C"))
  (bind _returnvalue_2 (Actor|GetComponentbyClass _owner "/Game/BP_Stubby/Blueprint_Components/BPC_Health.BPC_Health_C"))
  (bind _returnvalue_3 (Actor|GetComponentbyClass _owner_2 "/Script/UMG.WidgetComponent"))
  (bind _returnvalue_4 (UserInterface|GetWidget _returnvalue_3))
  (Utilities|IsValid _returnvalue_2
    (:Is%20Valid
      (Variables|/Game/BP_Stubby/Blueprint_Components/BPC_Health.BPC_Health_C|SetHealth _returnvalue_2 (- (Variables|/Game/BP_Stubby/Blueprint_Components/BPC_Health.BPC_Health_C|GetHealth _returnvalue_2) (Variables|Default|GetDamageAmount)))
      (Utilities|IsValid _returnvalue
        (:Is%20Valid
          (Utilities|IsValid _returnvalue_4
            (:Is%20Valid
              (bind _aswbp_enemy_health (Utilities|Casting|CastToWBP_EnemyHealth _returnvalue_4))
              (Utilities|IsValid _aswbp_enemy_health
                (:Is%20Valid
                  (Default|UpdateHealth _aswbp_enemy_health)
                  (Default|Death _returnvalue))))))))))

(event EventBeginPlay
  (Variables|Default|SetDamageAmount (Variables|Default|GetDamageAmount))
  (Variables|Default|SetOwner (Components|GetOwner)))