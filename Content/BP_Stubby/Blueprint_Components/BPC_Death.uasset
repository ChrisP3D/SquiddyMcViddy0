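; BPC_Death is an actor component that destroys its owning actor when its health runs out.
; It caches the owner on BeginPlay and exposes a Death event.
; When called, Death looks up the owner's BPC_Health component and destroys the owner only if that component exists and its Health is at or below zero.
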(event Custom|Death
  (bind _owner (Variables|Default|GetOwner))
  (bind _returnvalue (Actor|GetComponentbyClass _owner "/Game/BP_Stubby/Blueprint_Components/BPC_Health.BPC_Health_C"))
  (Utilities|IsValid _returnvalue
    (:Is%20Valid
      (if (<= (Variables|/Game/BP_Stubby/Blueprint_Components/BPC_Health.BPC_Health_C|GetHealth _returnvalue) 0.0)
        (Actor|DestroyActor (Variables|Default|GetOwner))))))

(event EventBeginPlay
  (Variables|Default|SetOwner (Components|GetOwner)))