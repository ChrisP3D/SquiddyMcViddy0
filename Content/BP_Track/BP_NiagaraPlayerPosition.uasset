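; BP_NiagaraPlayerPosition is an actor that feeds the player pawn's position into a Niagara system on a referenced rail attachment object.
; On BeginPlay it finds that object's NiagaraComponent and sets the player pawn as the system's User.BPCallback object.
; Every Tick, while the component is valid, it pushes the pawn's world location into the User.PlayerPawnPositionVector parameter.
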(event EventBeginPlay
  (bind _output_get (Variables|Default|SetRailAttachmentNiagaraSystemComponent (Actor|GetComponentbyClass (Variables|Default|GetRailAttachmentObject) "/Script/Niagara.NiagaraComponent")))
  (Class|NiagaraComponent|SetVariableObject _output_get "User.BPCallback" (Game|Player|GetPlayerPawn 0)))

(event Collision|EventActorBeginOverlap
  (params (OtherActor :type Actor%20Object%20Reference)))

(event EventTick
  (params (DeltaSeconds :type Float%20%28single-precision%29))
  (bind _railattachmentniagarasystemcomponent (Variables|Default|GetRailAttachmentNiagaraSystemComponent))
  (Utilities|IsValid _railattachmentniagarasystemcomponent
    (:Is%20Valid
      (Effects|Components|ParticleSystem|SetVectorParameter _railattachmentniagarasystemcomponent "User.PlayerPawnPositionVector" (Transformation|GetActorLocation (Game|Player|GetPlayerPawn 0))))))

(fn ConstructionScript)