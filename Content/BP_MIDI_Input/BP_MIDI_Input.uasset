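; MIDI input hub actor that discovers connected devices, creates an input controller for each by name, and spawns a CVThing monitor HUD at BeginPlay.
; Menu-picked devices bind to four slots storing control-change data in structs; only slot 0 forwards to the player pawn.
; Dedicated CVThing and Traktor-style "F1" handlers normalize CCs for HUD and pawn, with feedback to F1, but their device setup chain is disconnected from startup.
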(event Custom|BeginPlayInitCVThingCCsArray
  ;[1 0.1144 0.08228] INIT EMPTY CVTHING CCS ARRAY
  (for _index (range 0 (- (Variables|Default|GetNumControlsCVThing) 1))
    (Utilities|Array|SetArrayElem (Variables|Default|GetCVThingCCs) _index 0.0 true))
  ;[1 0.1144 0.08228] ADD HUD TO MONITOR CVTHING VALUES
  (bind _returnvalue (UserInterface|CreateWidget "/Game/WBP_HUD/WBP_HUD_Master_0.WBP_HUD_Master_0_C" (Game|GetPlayerController 0)))
  (bind _output_get (Variables|Default|SetCVThingHUD _returnvalue))
  (Variables|/Game/WBP_HUD/WBP_HUD_Master_0.WBP_HUD_Master_0_C|SetBP_MIDI_Input _output_get self)
  (UserInterface|Viewport|AddtoViewport _output_get 0))

(event Custom|GetCVThingMIDICCs
  (params (MIDIDeviceController :type MIDI%20Device%20Input%20Controller%20Object%20Reference) (Timestamp :type Integer) (Channel :type Integer) (Type :type Integer) (Value :type Integer))
  ;[1 0.1137 0.08235] GET ALL CV THING MIDI CC EVENTS, CAN FILTER THESE TO GET THE CC WE WANT
  (Variables|Default|SetTimestamp_CVThing Timestamp)
  (Variables|Default|SetChannel_CVThing Channel)
  (Variables|Default|SetType_CVThing Type)
  (Variables|Default|SetValue_CVThing Value)
  (Utilities|IsValid MIDIDeviceController
    (:Is%20Valid
      ;[1 0.1144 0.08228] LOOP AROUND NUM CONTROLS AND SET ARRAY
      (for _index (range 0 (- (Variables|Default|GetNumControlsCVThing) 1))
        (if (== (Variables|Default|GetType_CVThing) _index)
          (Utilities|Array|SetArrayElem (Variables|Default|GetCVThingCCs) _index (Math|Float|MapRangeClamped (Math|Conversions|ToFloat(Integer) (Variables|Default|GetValue_CVThing)) 0.0 127.0 0.0 1.0) true)))
      ;[1 0.1144 0.08228] PASS ENTIRES ARRAY OUT TO CV THING HUD USING BLUEPRINT INTERFACE MESSAGE
      (Class|BPIMIDI|ParseCVThingCCArray(Message) (Variables|Default|GetCVThingHUD) (Variables|Default|GetCVThingCCs)))))

(event Custom|BindCVThingCCEvents
  ;[1 0.1137 0.08235] BIND EVENTS TO CVTHING MIDI CC INPUT
  (EventDispatchers|BindEventtoOnMIDIControlChange (Variables|MIDI|GetCVThingInputController) (EventDispatchers|CreateEvent :!event GetCVTHingMIDICCs)))

(event Custom|SetCVThingInputController
  ;[1 0.1137 0.08235] SET CVTHING MIDI DEVICE INPUT CONTROLLER
  (bind _returnvalue (Class|MIDIDeviceManager|CreateMIDIDeviceInputController (Variables|MIDI|GetCVThingID) 1024))
  (Utilities|IsValid _returnvalue
    (:Is%20Valid
      (Variables|MIDI|SetCVThingInputController _returnvalue)
      ;[1 0.1137 0.08235] BIND EVENTS TO CVTHING MIDI CC INPUT
      (EventDispatchers|BindEventtoOnMIDIControlChange (Variables|MIDI|GetCVThingInputController) (EventDispatchers|CreateEvent :!event GetCVTHingMIDICCs)))))

(event Custom|BeginPlayFindAllMIDIDevices
  ;[1 1 1] MAKE AN ARRAY OF ALL MIDI DEVICES CURRENTLY CONNECTED TO COMPUTER
  (bind _outmididevices (Class|MIDIDeviceManager|FindMIDIDevices))
  (Variables|MIDI|SetOut%20MIDIDevices _outmididevices))

(event Custom|SetF1InputController
  ;[0 0 0] SET F1 INPUT CONTROLLER
  (bind _returnvalue (Class|MIDIDeviceManager|CreateMIDIDeviceInputController (Variables|Default|GetF1InputID) 1024))
  (Utilities|IsValid _returnvalue
    (:Is%20Valid
      (Variables|MIDI|SetF1InputController _returnvalue)
      ;[0 0 0] BIND EVENTS TO INCOMING F1 MIDI CCs
      (EventDispatchers|BindEventtoOnMIDIControlChange (Variables|MIDI|GetF1InputController) (EventDispatchers|CreateEvent :!event Custom|GetF1MIDICCs)))))

(event Custom|GetF1MIDICCs
  (params (MIDIDeviceController :type MIDI%20Device%20Input%20Controller%20Object%20Reference) (Timestamp :type Integer) (Channel :type Integer) (Type :type Integer) (Value :type Integer))
  ;[0 0 0 1 30] ON F1 MIDI CC EVENTS
  (Variables|Default|SetTimestamp_F1 Timestamp)
  (Variables|Default|SetChannel_F1 Channel)
  (Variables|Default|SetType_F1 Type)
  (Variables|Default|SetValue_F1 Value)
  (Utilities|IsValid MIDIDeviceController
    (:Is%20Valid
      ;[0 0 0] LOOP AROUND NUM CONTROLS AND SET ARRAY
      (for _index (range 0 (+ (Variables|Default|GetNumControlsF1) 1))
        (if (== (Variables|Default|GetType_F1) _index)
          (Utilities|Array|SetArrayElem (Variables|Default|GetF1CCs) _index (Math|Float|MapRangeClamped (Math|Conversions|ToFloat(Integer) (Variables|Default|GetValue_F1)) 0.0 127.0 0.0 1.0) true)))
      ;[0 0 0] PASS F1 CC EVENTS TO PLAYER PAWN
      (Class|BPIMIDI|ParseF1CCEvent(Message) (Game|Player|GetPlayerPawn 0) (Variables|Default|GetType_F1) 0 (Variables|Default|GetF1CCs)))))

(event Custom|GetMidiInput0
  (params (MIDIDeviceController :type MIDI%20Device%20Input%20Controller%20Object%20Reference) (Timestamp :type Integer) (Channel :type Integer) (Type :type Integer) (Value :type Integer))
  (bind _midicontrolchanges (Variables|Default|GetMidiControlChanges))
  (bind _midicontrolchanges_2 (Variables|Default|GetMidiControlChanges))
  (bind _output (Utilities|Array|Get(acopy) _midicontrolchanges))
  (bind _output_2 (Utilities|Array|Get(acopy) _midicontrolchanges_2))
  (bind _ccdata (Utilities|Struct|BreakSTR_MidiControlChange _output_2))
  (bind (_localid _firstindex _ncontrols) (Utilities|Struct|BreakSTR_MidiControlChange _output))
  (for _index (range _firstindex _ncontrols)
    (Utilities|Array|SetArrayElem _ccdata _index (Math|Float|MapRangeClamped (Math|Conversions|ToFloat(Integer) _index) 0.0 127.0 0.0 1.0) true)
    (bind _structout (Utilities|Struct|SetmembersinSTR_MidiControlChange _output_2 MIDIDeviceController Timestamp Channel Type Value _ccdata))
    (Class|BPIMIDI|ParseMidi(Message) (Game|Player|GetPlayerPawn 0) _structout)))

(event Custom|BeginPlayInitF1CCsArray
  ;[0 0 0] INIT EMPTY F1 CCS ARRAY
  (for _index (range 2 (+ (Variables|Default|GetNumControlsF1) 1))
    (Utilities|Array|SetArrayElem (Variables|Default|GetF1CCs) _index 0.0 true)))

(event Custom|GetMidiInput3
  (params (MIDIDeviceController :type MIDI%20Device%20Input%20Controller%20Object%20Reference) (Timestamp :type Integer) (Channel :type Integer) (Type :type Integer) (Value :type Integer))
  (Utilities|Struct|SetmembersinSTR_MidiControlChange (Utilities|Array|Get(acopy) (Variables|Default|GetMidiControlChanges) 3) MIDIDeviceController Timestamp Channel Type Value))

(event Custom|SetMidiDevice)

(event Custom|GetMidiInput1
  (params (MIDIDeviceController :type MIDI%20Device%20Input%20Controller%20Object%20Reference) (Timestamp :type Integer) (Channel :type Integer) (Type :type Integer) (Value :type Integer))
  (Utilities|Struct|SetmembersinSTR_MidiControlChange (Utilities|Array|Get(acopy) (Variables|Default|GetMidiControlChanges) 1) MIDIDeviceController Timestamp Channel Type Value))

(event Custom|GetMidiInput2
  (params (MIDIDeviceController :type MIDI%20Device%20Input%20Controller%20Object%20Reference) (Timestamp :type Integer) (Channel :type Integer) (Type :type Integer) (Value :type Integer))
  (Utilities|Struct|SetmembersinSTR_MidiControlChange (Utilities|Array|Get(acopy) (Variables|Default|GetMidiControlChanges) 2) MIDIDeviceController Timestamp Channel Type Value))

(event Custom|SetF1OutputController
  ;[0 0 0] SET F1 OUTPUT CONTROLLER
  (bind _returnvalue (Class|MIDIDeviceManager|CreateMIDIDeviceOutputController (Variables|Default|GetF1OutputID)))
  (Utilities|IsValid _returnvalue
    (:Is%20Valid
      (Variables|Default|SetF1OutputController _returnvalue))))

(event Custom|SetF1ID
  ;[0 0 0 1 30] SET F1 MIDI INPUT DEVICE ID
  ; USE CONTAINS F1
  (for _array_element (Variables|MIDI|GetOut%20MIDIDevices)
    (if (and (Utilities|String|Contains (.DeviceName (Utilities|Struct|BreakFoundMIDIDevice _array_element)) "F1") (.bCanReceiveFrom (Utilities|Struct|BreakFoundMIDIDevice _array_element)))
      (Variables|Default|SetF1InputID (.DeviceID (Utilities|Struct|BreakFoundMIDIDevice _array_element)))))
  ;[0 0 0 1 30] SET F1 MIDI INPUT DEVICE ID
  ; USE CONTAINS F1
  (for _array_element_2 (Variables|MIDI|GetOut%20MIDIDevices)
    (if (and (Utilities|String|Contains (.DeviceName (Utilities|Struct|BreakFoundMIDIDevice _array_element_2)) "F1") (not (.bCanReceiveFrom (Utilities|Struct|BreakFoundMIDIDevice _array_element_2))))
      (Variables|Default|SetF1OutputID (.DeviceID (Utilities|Struct|BreakFoundMIDIDevice _array_element_2)))
      ;[0 0 0] SET F1 INPUT CONTROLLER
      (Utilities|FlowControl|Sequence
        (:then_0
          (bind _returnvalue (Class|MIDIDeviceManager|CreateMIDIDeviceInputController (Variables|Default|GetF1InputID) 1024))
          (Utilities|IsValid _returnvalue
            (:Is%20Valid
              (Variables|MIDI|SetF1InputController _returnvalue)
              ;[0 0 0] BIND EVENTS TO INCOMING F1 MIDI CCs
              (EventDispatchers|BindEventtoOnMIDIControlChange (Variables|MIDI|GetF1InputController) (EventDispatchers|CreateEvent :!event Custom|GetF1MIDICCs)))))
        (:then_1
          ;[0 0 0] SET F1 OUTPUT CONTROLLER
          (bind _returnvalue_2 (Class|MIDIDeviceManager|CreateMIDIDeviceOutputController (Variables|Default|GetF1OutputID)))
          (Utilities|IsValid _returnvalue_2
            (:Is%20Valid
              (Variables|Default|SetF1OutputController _returnvalue_2))))))))

(event Custom|TrySetup
  (for _array_element (Variables|MIDI|GetOut%20MIDIDevices)
    (bind _returnvalue (Class|MIDIDeviceManager|CreateMIDIDeviceInputController (.DeviceID (Utilities|Struct|BreakFoundMIDIDevice _array_element)) 1024))
    (Utilities|Map|Add (Variables|Default|GetInputControllers) (.DeviceName (Utilities|Struct|BreakFoundMIDIDevice _array_element)) _returnvalue)))

(event Custom|SetCVThingID
  ;[1 0.1119 0.08228 1 30] SET CV THING MIDI INPUT DEVICE ID
  ; MATCH EXACT STRING, COULD USE CONTAINS 'THING'
  ; CAN RECEIVE FROM SPECIFIES IT IS AN INPUT
  (for _array_element (Variables|MIDI|GetOut%20MIDIDevices)
    (if (and (.bCanReceiveFrom (Utilities|Struct|BreakFoundMIDIDevice _array_element)) (Utilities|Enum|Equal(Enum) (.DeviceName (Utilities|Struct|BreakFoundMIDIDevice _array_element)) "CVThing"))
      (Variables|MIDI|SetCVThingID (.DeviceID (Utilities|Struct|BreakFoundMIDIDevice _array_element)))
      ;[1 0.1137 0.08235] SET CVTHING MIDI DEVICE INPUT CONTROLLER
      (bind _returnvalue (Class|MIDIDeviceManager|CreateMIDIDeviceInputController (Variables|MIDI|GetCVThingID) 1024))
      (Utilities|IsValid _returnvalue
        (:Is%20Valid
          (Variables|MIDI|SetCVThingInputController _returnvalue)
          ;[1 0.1137 0.08235] BIND EVENTS TO CVTHING MIDI CC INPUT
          (EventDispatchers|BindEventtoOnMIDIControlChange (Variables|MIDI|GetCVThingInputController) (EventDispatchers|CreateEvent :!event GetCVTHingMIDICCs)))))))

(event Custom|BindF1CCEvents
  ;[0 0 0] BIND EVENTS TO INCOMING F1 MIDI CCs
  (EventDispatchers|BindEventtoOnMIDIControlChange (Variables|MIDI|GetF1InputController) (EventDispatchers|CreateEvent :!event Custom|GetF1MIDICCs)))

(event EventParseF1CCEvent
  (params (F1CCType :type Integer) (F1CCValue :type Integer) (F1CCs :type Array%20of%20Floats%20%28double-precision%29))
  ;[0 0 0 1 36] SEND MIDI EVENTS BACK TO F1
  (Class|MIDIDeviceOutputController|SendMIDIControlChange (Variables|Default|GetF1OutputController) 12 11 (Math|Conversions|ToInteger(Byte) (Class|KismetMathLibrary|ToInt64(Float) (Math|Float|MapRangeClamped (Utilities|Array|Get(acopy) (Variables|Default|GetCVThingCCs) 3) 0.0 1.0 0.0 127.0)))))

(event EventInitMidi
  ;[0.6373 0.5586 1 1 40] BEGIN PLAY
  ;;[1 1 1] CPs addition
  (Utilities|FlowControl|Sequence
    (:then_0
      (CallFunction|BeginPlayFindAllMIDIDevices)
      (CallFunction|SetMidiDeviceNames)
      (for _array_element (Variables|MIDI|GetOut%20MIDIDevices)
        _))
    (:then_1
      (CallFunction|TrySetup)
      (CallFunction|BeginPlayInitCVThingCCsArray)
      (CallFunction|BeginPlayInitF1CCsArray))))

(event EventBeginPlay
  ;[0.6373 0.5586 1 1 40] BEGIN PLAY
  ;;[1 1 1] CPs addition
  (Utilities|FlowControl|Sequence
    (:then_0
      (CallFunction|BeginPlayFindAllMIDIDevices)
      (CallFunction|SetMidiDeviceNames)
      (for _array_element (Variables|MIDI|GetOut%20MIDIDevices)
        _))
    (:then_1
      (CallFunction|TrySetup)
      (CallFunction|BeginPlayInitCVThingCCsArray)
      (CallFunction|BeginPlayInitF1CCsArray))))

(event EventSetNewMidiDevice
  (params (Device%20Info :type STR%20Midi%20Device%20Info%20Structure) (LocalID :type Integer) (NControls :type Integer))
  (bind (_deviceid _devicename _cansendto _isalreadyinuse _isdefaultinputdevice _isdefaultoutputdevice _ncontrols) (Utilities|Struct|BreakSTR_MidiDeviceInfo Device%20Info))
  (bind _inputcontrollers (Variables|Default|GetInputControllers))
  (bind _devicenames (Variables|Default|GetDeviceNames))
  (bind _devicenames_2 (Variables|Default|GetDeviceNames))
  (bind _returnvalue (Utilities|Array|FindItem _devicenames_2 _devicename))
  (bind _output (Utilities|Array|Get(acopy) _devicenames _returnvalue))
  (bind (_value _returnvalue_2) (Utilities|Map|Find _inputcontrollers _output))
  ;[1 1 1] Picked From List Of Devices in Midi Menu
  (Utilities|FlowControl|Sequence
    (:then_0
      (if (> _returnvalue -1)
        (if _returnvalue_2
          (Utilities|IsValid _value
            (:Is%20Valid
              (Utilities|FlowControl|Sequence
                (:then_0
                  (Utilities|Struct|SetmembersinSTR_MidiControlChange (Utilities|Array|Get(acopy) (Variables|Default|GetMidiControlChanges) LocalID) LocalID))
                (:then_1
                  (switch int LocalID
                    (:0
                      (EventDispatchers|BindEventtoOnMIDIControlChange _value (EventDispatchers|CreateEvent :!event Custom|GetMidiInput0)))
                    (:1
                      (EventDispatchers|BindEventtoOnMIDIControlChange _value (EventDispatchers|CreateEvent :!event Custom|GetMidiInput1)))
                    (:2
                      (EventDispatchers|BindEventtoOnMIDIControlChange _value (EventDispatchers|CreateEvent :!event Custom|GetMidiInput2)))
                    (:3
                      (EventDispatchers|BindEventtoOnMIDIControlChange _value (EventDispatchers|CreateEvent :!event Custom|GetMidiInput3)))))))
            (:Is%20Not%20Valid
              (Development|PrintString "Midi Input Controller Found Indide \"InputControllers*MAP*)\" is not Vliad" true true "(R=1.000000,G=0.000000,B=0.000000,A=1.000000)"))))
        (else
          (Development|PrintString "Device Not Found"))))
    (:then_1
      (if (> _ncontrols -1)
        (Utilities|Struct|SetmembersinSTR_MidiControlChange (Utilities|Array|Get(acopy) (Variables|Default|GetMidiControlChanges) LocalID) _ncontrols)))))

(event Input|KeyboardEvents|DebugKey1
  (params (Key :type Key%20Structure :default "None") (ActionValue :type Input%20Action%20Value%20Structure))
  (:Pressed
    (bind _returnvalue (Actor|GetActorOfClass "BP_MIDI_Input_C"))
    (for _array_element (Variables|BP_MIDI_Input_C|GetDeviceNames _returnvalue)
      (Development|PrintString _array_element))))

(fn ConstructionScript)

(fn FoundMidiDevices
  (return (> (Utilities|Array|Length (Variables|MIDI|GetOut%20MIDIDevices)) 0)))

(fn SetMidiDeviceNames
  (for _array_element (Variables|MIDI|GetOut%20MIDIDevices)
    (Utilities|Array|AddUnique (Variables|Default|GetDeviceNames) (.DeviceName (Utilities|Struct|BreakFoundMIDIDevice _array_element)))))

(fn BPMIDIInputAutoGenFunc
  (params (MIDIDeviceController :type MIDI%20Device%20Input%20Controller%20Object%20Reference) (Timestamp :type Integer) (Channel :type Integer) (Type :type Integer) (Value :type Integer)))

(fn GetDeviceNames
  (return (Variables|Default|GetDeviceNames)))

(fn GetDevices
  (return (Variables|MIDI|GetOut%20MIDIDevices) 0))

(fn InitializeCVThingCCArray
  (return (Variables|Default|GetCVThingCCs)))

(fn ParseCVThingCCValue
  (params (FiltterCC# :type Integer%20%28by%20ref%29) (InputType :type Integer%20%28by%20ref%29) (InputValue :type Integer%20%28by%20ref%29))
  (return 0.0))

(fn ParseF1CCValue
  (params (FilterCC# :type Integer) (InputType :type Integer) (InputValue :type Integer))
  (return 0.0))