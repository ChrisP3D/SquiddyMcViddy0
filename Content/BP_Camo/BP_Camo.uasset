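; BP_Camo is a camera rig Blueprint that pairs a SpringArm with a CineCamera and is driven through a CameraControl interface event.
; The event sets the arm's world rotation and length, then the camera's focal length and aperture.
; It then applies manual focus at the measured distance from the camera to the player pawn, recalculated on each call.
; Tick, BeginPlay and the construction script contain no logic.
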(event EventBeginPlay)

(event Collision|EventActorBeginOverlap
  (params (OtherActor :type Actor%20Object%20Reference)))

(event EventTick
  (params (DeltaSeconds :type Float%20%28single-precision%29)))

(event EventCameraControl
  (params (TargetArmAddRotation :type Rotator :default "0, 0, 0") (TargetArmLength :type Float%20%28double-precision%29) (CameraFocalLength :type Float%20%28double-precision%29) (CameraAperture :type Float%20%28double-precision%29) (CameraFocusDistance :type Float%20%28double-precision%29))
  ;[0.1471 0.2552 0.1004] CAMERA CONTROL INTERFACE
  (Transformation|SetWorldRotation (Variables|Default|GetSpringArm) TargetArmAddRotation false false)
  (Variables|/Script/Engine.SpringArmComponent|SetTargetArmLength (Variables|Default|GetSpringArm) TargetArmLength)
  (Variables|/Script/CinematicCamera.CineCameraComponent|SetCurrentFocalLength (Variables|Default|GetCineCamera) CameraFocalLength)
  (Variables|/Script/CinematicCamera.CineCameraComponent|SetCurrentAperture (Variables|Default|GetCineCamera) CameraAperture)
  (Variables|/Script/CinematicCamera.CineCameraComponent|SetFocusSettings (Variables|Default|GetCineCamera) (Utilities|Struct|MakeCameraFocusSettings "Manual" (Math|Vector|VectorLength (- (Transformation|GetWorldLocation (Variables|Default|GetCineCamera)) (Transformation|GetActorLocation (Game|Player|GetPlayerPawn 0)))) "(ActorToTrack=None,RelativeOffset=(X=0.000000,Y=0.000000,Z=0.000000))" false 1.0 0.0)))

(fn ConstructionScript)